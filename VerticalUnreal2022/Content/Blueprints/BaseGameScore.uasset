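; BaseGameScore runs the match countdown timer and ends the game when time runs out.
; On BeginPlay it adds the BaseGame_UI widget to the viewport.
; Tick passes through a one-second Delay to count down Minutes and Seconds, using the latent node as a timer.
; At zero it shows GameOver_UI, hides the mouse cursor and pauses the game.
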(event EventBeginPlay
  (bind _returnvalue (UserInterface|CreateWidget "/Game/Blueprints/BaseGame_UI.BaseGame_UI_C"))
  (UserInterface|Viewport|AddtoViewport _returnvalue 0))

(event EventTick
  (params (DeltaSeconds :type Float%20%28single-precision%29))
  (Utilities|FlowControl|Delay 1.0)
  (if (== (Variables|Default|GetSeconds) 0)
    (if (== (Variables|Default|GetMinutes) 0)
      (bind _returnvalue (UserInterface|CreateWidget "/Game/Blueprints/GameOver_UI.GameOver_UI_C"))
      (UserInterface|Viewport|AddtoViewport _returnvalue 0)
      (Variables|/Script/Engine.PlayerController|SetbShowMouseCursor (Game|GetPlayerController 0) false)
      (Game|SetGamePaused true)
      (else
        (Variables|Default|SetSeconds 59)
        (Variables|Default|SetMinutes (- (Variables|Default|GetMinutes) 1))))
    (else
      (Variables|Default|SetSeconds (- (Variables|Default|GetSeconds) 1)))))

(fn ConstructionScript)