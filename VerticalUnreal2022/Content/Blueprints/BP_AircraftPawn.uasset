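; Player aircraft pawn with mouse-aim flight, where the plane steers itself toward the point the player aims at.
; Mouse input rotates an aim scene that the camera rig follows with exponential damping.
; An autopilot derives yaw, pitch and roll, blending wings-level into aggressive banking, with manual pitch and roll overrides.
; Each tick applies thrust and torque to the mesh and projects boresight and aim markers onto the HUD.
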(event Custom|Update%20HUD
  (Utilities|FlowControl|Sequence
    (:then_0
      (Default|SetBoresightImagePosition (Variables|Runtime|GetHUD%20Reference) (.ScreenPosition (Class|WidgetLayoutLibrary|ProjectWorldLocationtoWidgetPosition (Game|GetPlayerController 0) (CallFunction|GetBoresightEndLocation) false))))
    (:then_1
      (Default|SetAimImagePosition (Variables|Runtime|GetHUD%20Reference) (.ScreenPosition (Class|WidgetLayoutLibrary|ProjectWorldLocationtoWidgetPosition (Game|GetPlayerController 0) (CallFunction|GetControllerAimEndLocation) false))))))

(event Custom|Update%20Physics
  (CallFunction|UpdateAircraftPhysics))

(event Custom|Rotate%20Rig
  (params (Input%20X :type Float%20%28double-precision%29) (Input%20Y :type Float%20%28double-precision%29))
  (bind _camerarig_scene (Variables|Default|GetCameraRig_Scene))
  (Transformation|AddWorldRotation (Variables|Default|GetControllerAim_Scene) (Math|Vector|RotatorfromAxisandAngle (Math|Vector|GetUpVector (Variables|Default|GetMainCamera)) Input%20X) false false)
  (Transformation|AddWorldRotation (Variables|Default|GetControllerAim_Scene) (Math|Vector|RotatorfromAxisandAngle (Math|Vector|GetRightVector (Variables|Default|GetMainCamera)) Input%20Y) false false)
  (Transformation|SetWorldRotation (Variables|Default|GetCameraRig_Scene) (CallFunction|Damp (Transformation|GetWorldRotation (Variables|Default|GetCameraRig_Scene)) (Math|Rotator|MakeRotfromXZ (- (CallFunction|GetControllerAimEndLocation) (Transformation|GetWorldLocation _camerarig_scene)) (select (> (.Z (Math|Vector|BreakVector (Math|Vector|GetForwardVector (Variables|Default|GetControllerAim_Scene)))) 0.9) (Math|Vector|GetUpVector _camerarig_scene) (Math|Vector|MakeVector 0.0 0.0 1.0))) (Variables|Default|GetCamera%20Smooth%20Speed) (Variables|Default|GetDelta%20Seconds) true) false false))

(event EventBeginPlay
  (bind _returnvalue (UserInterface|CreateWidget "/Game/Blueprints/WG_GameHUD.WG_GameHUD_C"))
  (bind _output_get (Variables|Runtime|SetHUD%20Reference _returnvalue))
  (UserInterface|Viewport|AddtoViewport _output_get 0)
  (Transformation|SetAbsolute (Variables|Default|GetController_ROOT) false true true))

(event EventTick
  (params (DeltaSeconds :type Float%20%28single-precision%29))
  (Variables|Default|SetDelta%20Seconds DeltaSeconds)
  (CallFunction|UpdatePhysics)
  (CallFunction|UpdateHUD))

(event Input|AxisEvents|InputAxisLookUp
  (params (AxisValue :type Float%20%28single-precision%29))
  (CallFunction|RotateRig 0.0 (* AxisValue (Variables|Default|GetMouse%20Sensivity))))

(event Input|AxisEvents|InputAxisLookRight
  (params (AxisValue :type Float%20%28single-precision%29))
  (CallFunction|RotateRig (* (Variables|Default|GetMouse%20Sensivity) AxisValue) 0.0))

(fn ConstructionScript)

(fn GetBoresightEndLocation
  (return (+ (Transformation|GetActorLocation) (* (Transformation|GetActorForwardVector) (Variables|Default|GetAim%20Distance)))))

(fn GetControllerAimEndLocation
  (bind _controlleraim_scene (Variables|Default|GetControllerAim_Scene))
  (return (+ (Transformation|GetWorldLocation _controlleraim_scene) (* (Math|Vector|GetForwardVector _controlleraim_scene) (Variables|Default|GetAim%20Distance)))))

(fn GetBoresightStartLocation
  (return (Transformation|GetActorLocation)))

(fn GetControllerAimStartLocation
  (return (Transformation|GetWorldLocation (Variables|Default|GetControllerAim_Scene))))

(fn Damp
  (params (A :type Rotator) (B :type Rotator) (Lambda%20Time :type Float%20%28double-precision%29) (Delta%20Seconds :type Float%20%28double-precision%29) (Shortest%20Path :type Boolean))
  (return (Math|Rotator|Lerp(Rotator) A B (* 1.0 (Class|KismetMathLibrary|Exp (* Lambda%20Time Delta%20Seconds -1.0))) Shortest%20Path)))

(fn RunAutopilot
  (params (Fly%20Target :type Vector) (Out%20Yaw :type Float%20%28double-precision%29) (Out%20Pitch :type Float%20%28double-precision%29) (Out%20Roll :type Float%20%28double-precision%29))
  (Utilities|FlowControl|Sequence
    (:then_0
      (LocalVariables|SetLocal%20Fly%20Target (* (Math|Vector|Normalize (Math|Transform|InverseTransformLocation (Transformation|GetActorTransform) Fly%20Target)) (Variables|Default|GetSensivity)))
      (LocalVariables|SetAngle%20Off%20Target (Class|KismetMathLibrary|DegAcos (Math|Vector|DotProduct (Transformation|GetActorForwardVector) (Math|Vector|Normalize (- Fly%20Target (Transformation|GetActorLocation)))))))
    (:then_1
      (|SetBy-RefVar Out%20Yaw (Math|Float|Clamp(Float) (.Y (Math|Vector|BreakVector (LocalVariables|GetLocal%20Fly%20Target))) -1.0))
      (|SetBy-RefVar Out%20Pitch (Math|Float|Clamp(Float) (.Z (Math|Vector|BreakVector (LocalVariables|GetLocal%20Fly%20Target))) -1.0)))
    (:then_2
      (LocalVariables|SetAggressive%20Roll (Math|Float|Clamp(Float) (.Y (Math|Vector|BreakVector (LocalVariables|GetLocal%20Fly%20Target))) -1.0))
      (LocalVariables|SetWings%20Level%20Roll (.Z (Math|Vector|BreakVector (Transformation|GetActorRightVector))))
      (LocalVariables|SetWings%20Level%20Influence (Math|Float|Clamp(Float) (Math|Float|NormalizetoRange (LocalVariables|GetAngle%20Off%20Target) 0.0 (Variables|Default|GetAggressive%20Turn%20Angle))))
      (|SetBy-RefVar Out%20Roll (Math|Float|Lerp (LocalVariables|GetWings%20Level%20Roll) (LocalVariables|GetAggressive%20Roll) (LocalVariables|GetWings%20Level%20Influence))))))

(fn UpdateAircraftPhysics
  (Utilities|FlowControl|Sequence
    (:then_0
      (LocalVariables|SetRoll%20Override false)
      (LocalVariables|SetPitch%20Override false)
      (LocalVariables|SetAuto%20Yaw 0.0)
      (LocalVariables|SetAuto%20Pitch 0.0)
      (LocalVariables|SetAuto%20Roll 0.0))
    (:then_1
      (Utilities|FlowControl|Sequence
        (:then_0
          (if (> (Math|Float|Absolute(Float) (Input|AxisValues|GetRollAxis)) 0.25)
            (LocalVariables|SetRoll%20Override true)))
        (:then_1
          (if (> (Math|Float|Absolute(Float) (Input|AxisValues|GetPitchAxis)) 0.25)
            (LocalVariables|SetRoll%20Override true)
            (LocalVariables|SetPitch%20Override true)))))
    (:then_2
      (CallFunction|RunAutopilot (CallFunction|GetControllerAimEndLocation) (LocalVariables|GetAuto%20Yaw) (LocalVariables|GetAuto%20Pitch) (LocalVariables|GetAuto%20Roll)))
    (:then_3
      (LocalVariables|SetCurrent%20Yaw (LocalVariables|GetAuto%20Yaw))
      (LocalVariables|SetCurrent%20Pitch (select (LocalVariables|GetPitch%20Override) (Input|AxisValues|GetPitchAxis) (LocalVariables|GetAuto%20Pitch)))
      (LocalVariables|SetCurrent%20Roll (select (LocalVariables|GetRoll%20Override) (Input|AxisValues|GetRollAxis) (LocalVariables|GetAuto%20Roll))))
    (:then_4
      (Utilities|FlowControl|Sequence
        (:then_0
          (Physics|AddForce (Variables|Default|GetSM_Aircraft) (* (Transformation|GetActorForwardVector) (* (Variables|Default|GetThrust) (Variables|Default|GetForce%20Multiplier))) "None" false))
        (:then_1
          (Class|PrimitiveComponent|AddTorqueinRadians (Variables|Default|GetSM_Aircraft) (* (Math|Transform|TransformDirection (Transformation|GetActorTransform) (* (Variables|Default|GetTurn%20Torque) (Math|Vector|MakeVector (LocalVariables|GetCurrent%20Roll) (LocalVariables|GetCurrent%20Pitch) (LocalVariables|GetCurrent%20Yaw)))) (Variables|Default|GetForce%20Multiplier)) "None" false))))))