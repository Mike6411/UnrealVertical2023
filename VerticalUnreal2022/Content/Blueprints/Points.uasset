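; Points is a scoring actor that awards points and destroys itself when a bullet or the player overlaps it.
; On begin overlap, a sequence checks the other actor for the Bullet and Player tags, with player contact worth more than a bullet hit.
; Each matching branch finds the BaseGameScore actor by class, adds directly to its Points variable, then destroys this actor.
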(event Collision|EventActorBeginOverlap
  (params (OtherActor :type Actor%20Object%20Reference))
  (Utilities|FlowControl|Sequence
    (:then_0
      (if (Actor|ActorHasTag OtherActor "Bullet")
        (bind _returnvalue (Actor|GetActorOfClass "/Game/Blueprints/BaseGameScore.BaseGameScore_C"))
        (bind _asbase_game_score (Utilities|Casting|CastToBaseGameScore _returnvalue))
        (Variables|/Game/Blueprints/BaseGameScore.BaseGameScore_C|SetPoints _asbase_game_score (+ (Variables|/Game/Blueprints/BaseGameScore.BaseGameScore_C|GetPoints _asbase_game_score) 1e+02))
        (Actor|DestroyActor)))
    (:then_1
      (if (Actor|ActorHasTag OtherActor "Player")
        (bind _returnvalue_2 (Actor|GetActorOfClass "/Game/Blueprints/BaseGameScore.BaseGameScore_C"))
        (bind _asbase_game_score_2 (Utilities|Casting|CastToBaseGameScore _returnvalue_2))
        (Variables|/Game/Blueprints/BaseGameScore.BaseGameScore_C|SetPoints _asbase_game_score_2 (+ (Variables|/Game/Blueprints/BaseGameScore.BaseGameScore_C|GetPoints _asbase_game_score_2) 5e+02))
        (Actor|DestroyActor)))))

(fn ConstructionScript)