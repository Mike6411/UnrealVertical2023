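; Player-controlled jet fighter pawn that taxis, takes off, flies and lands, with a rechargeable nitro boost.
; IsFlying switches the input axes between ground taxi with camera look and interpolated thrust, pitch, yaw and roll driving swept offsets and control-surface rotations.
; A downward trace lands the jet at low throttle.
; Tick also scales exhaust effects, updates nitro, and feeds the Jet_UI HUD's speed, altitude, crosshair and roll indicators.
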(event EventBeginPlay
  ;[1 1 1] Begin play
  (Utilities|FlowControl|Sequence
    (:then_0
      (Variables|Speed|SetTarget%20thrust%20speed (Variables|Speed|GetMinimum%20thrust%20speed))
      (Variables|Default|SetStart%20Z%20Offset 1.2e+02)
      ;;[1 1 1] Creacion y añado del HUD
      (bind _returnvalue (UserInterface|CreateWidget "/Game/Assets/Jet/HUD/Jet_UI.Jet_UI_C"))
      (bind _output_get (Variables|Default|SetHUD%20Ref _returnvalue))
      (UserInterface|Viewport|AddtoViewport _output_get 0))
    (:then_1
      (Transformation|SetRelativeScale3D (Variables|Default|GetLeft_Exhaust) "0, 0, 0"))))

(event EventTick
  (params (DeltaSeconds :type Float%20%28single-precision%29))
  ;[1 1 1] Tick
  (Utilities|FlowControl|Sequence
    (:then_0
      ;;[1 1 1] Movimiento en el suelo con un interp para que accelere muy lentamente
      (bind _output_get (Variables|Default|SetMove%20Forward%20Interp (Math|Float|Clamp(Float) (Math|Interpolation|FInterpTo (stale _output_get) (Input|AxisValues|GetMoveForward) (Utilities|Time|GetWorldDeltaSeconds) 0.0))))
      ;;[1 1 1] Seteando el tamaño del fuego de escape
      (Transformation|SetRelativeScale3D (Variables|Default|GetRight_Exhaust) (Math|Interpolation|VInterpTo (Variables|/Script/Engine.SceneComponent|GetRelativeScale3D (Variables|Default|GetLeft_Exhaust)) (Math|Vector|SelectVector (Math|Vector|MakeVector (Math|Float|NormalizetoRange (Variables|Speed|GetCurrent%20thrust%20speed) 0.0 (Variables|Speed|GetMaximum%20thrust%20speed)) (Math|Float|NormalizetoRange (Variables|Speed|GetCurrent%20thrust%20speed) 0.0 (Variables|Speed|GetMaximum%20thrust%20speed)) (Math|Float|NormalizetoRange (Variables|Speed|GetCurrent%20thrust%20speed) 0.0 (Variables|Speed|GetMaximum%20thrust%20speed))) "0, 0, 0" (Variables|Default|GetIsFlying?)) (Utilities|Time|GetWorldDeltaSeconds) (Math|Float|SelectFloat 4.0 0.5 (Variables|Default|GetIsFlying?)))))
    (:then_1
      ;;[1 1 1] Flight check
      (if (Variables|Default|GetIsFlying?)
        (CallFunction|AddFlightMovement)
        (CallFunction|LandingTrace "ForOneFrame" (Variables|Default|GetStart%20Z%20Offset))))
    (:then_2
      (|HUDGRAPH))
    (:then_3
      (Utilities|SetAltitudeLevel))
    (:then_4
      ;;[1 1 1] Si se esta usando el boost que se consuma si no que se llena. Se llena mas rapido de lo que se consume.
      (Utilities|FlowControl|Sequence
        (:then_0
          (bind _output_get_2 (Variables|Nitro|SetNitro%20Level (Math|Interpolation|FInterpTo (stale _output_get_2) (Math|Float|SelectFloat 0.0 1.0 (Variables|Nitro|GetIsNitro?)) (Utilities|Time|GetWorldDeltaSeconds) (Math|Float|SelectFloat 0.1 0.05 (Variables|Nitro|GetIsNitro?)))))
          (Progress|SetPercent (Variables|/Game/Assets/Jet/HUD/Jet_UI.Jet_UI_C|GetNitroBar (Variables|Default|GetHUD%20Ref)) _output_get_2)
          (if (== _output_get_2 0.0)
            (bind _output_get_3 (Variables|Speed|SetMaximum%20thrust%20speed 2.5e+04))
            (Variables|Speed|SetTarget%20thrust%20speed _output_get_3)
            (Variables|Nitro|SetIsNitro? false)
            (Class|NiagaraComponent|SetAsset (Variables|Default|GetLeft_Exhaust) "/Game/Assets/Jet/VFX/JetExhaust_NS.JetExhaust_NS" true)))))))

(event Input|ActionEvents|InputActionBoost
  (params (Key :type Key%20Structure :default "None"))
  ;[1 1 1] Si el boost esta al maximo y se le da al input activamos el boost
  (:Pressed
    (if (and (== (Variables|Nitro|GetNitro%20Level) 1.0) (Variables|Default|GetIsFlying?))
      (Variables|Nitro|SetIsNitro? true)
      (bind _output_get (Variables|Speed|SetMaximum%20thrust%20speed (Variables|Nitro|GetNitro%20Thrust%20Speed)))
      (bind _output_get_2 (Variables|Speed|SetTarget%20thrust%20speed _output_get))
      (Variables|Speed|SetCurrent%20thrust%20speed _output_get_2)
      (Effects|SpawnEmitterAttached "/Game/Assets/Jet/VFX/Ringburst_PS.Ringburst_PS" (Variables|Default|GetSK_West_Fighter_Typhoon) "None" "0, 0, 0" "0, 0, 0" "7.000000,7.000000,7.000000")
      (Class|NiagaraComponent|SetAsset (Variables|Default|GetLeft_Exhaust) "/Game/Assets/Jet/VFX/NitroExhaust_NS.NitroExhaust_NS" true))))

(event Input|AxisEvents|InputAxisMoveForward
  (params (AxisValue :type Float%20%28single-precision%29))
  (bind _wheel_rotation_side_max (Variables|MeshTransforms|GetWheel%20Rotation%20side%20max))
  ;[1 1 1] Move Forward
  ;;[1 1 1] Si esta volando el input accelerara o decelerara la velocidad. Si no, se mueve por el suelo usando el offset
  (if (Variables|Default|GetIsFlying?)
    (if (not (Variables|Nitro|GetIsNitro?))
      (Variables|Speed|SetTarget%20thrust%20speed (Math|Float|Clamp(Float) (+ (* AxisValue (Utilities|Time|GetWorldDeltaSeconds) 2.5e+03) (Variables|Speed|GetTarget%20thrust%20speed)) (Variables|Speed|GetMinimum%20thrust%20speed) (Variables|Speed|GetMaximum%20thrust%20speed)))
      (if (not (Variables|Default|GetIsFlying?)) :!label _label
        (Utilities|FlowControl|Sequence
          (:then_0
            ;;[1 1 1] Mover el jet por el suelo
            (Transformation|AddActorWorldOffset (Math|Vector|MakeVector (.X (Math|Vector|BreakVector (* (Transformation|GetActorForwardVector) (Variables|Default|GetMove%20Forward%20Interp) (/ (Variables|Speed|GetTarget%20thrust%20speed) 5e+02)))) (.Y (Math|Vector|BreakVector (* (Transformation|GetActorForwardVector) (Variables|Default|GetMove%20Forward%20Interp) (/ (Variables|Speed|GetTarget%20thrust%20speed) 5e+02)))) 0.0) true)
            ;;[1 1 1] Si se esta moviendo y se pulsa espacio el jet despega y pasa a volar. Le damos un pequeño offset para que no nos estimbemos justo al despegar
            (if (and (> (Variables|Default|GetMove%20Forward%20Interp) 0.7) (Game|Player|IsInputKeyDown (Game|GetPlayerController 0) "SpaceBar"))
              (Variables|Default|SetIsFlying? true)
              (Variables|/Script/Engine.SpringArmComponent|SetbUsePawnControlRotation (Variables|Default|GetSpringArm) false)
              (Transformation|AddActorWorldOffset "0, 0,35.000000" true)))
          (:then_1
            ;;[1 1 1] Set de la rotacion de la rueda para el forward y el side
            (Variables|MeshTransforms|SetWheel%20Rotation (Math|Rotator|MakeRotator 0.0 (+ (.pitch (Transformation|GetSocketRotation (Variables|Default|GetSK_West_Fighter_Typhoon) "front_wheel_jnt")) (* (Variables|Default|GetMove%20Forward%20Interp) -5e+02)) (Math|Interpolation|FInterpTo (.yaw (Variables|MeshTransforms|GetWheel%20Rotation)) (Math|Float|MapRangeClamped (Input|AxisValues|GetMoveRight) -1.0 1.0 (* _wheel_rotation_side_max -1.0) _wheel_rotation_side_max) (Utilities|Time|GetWorldDeltaSeconds) 0.4)))))))
    (else
      (goto _label))))

(event Input|AxisEvents|InputAxisLookUp
  (params (AxisValue :type Float%20%28single-precision%29))
  (bind _returnvalue (Utilities|Time|GetWorldDeltaSeconds))
  (bind _isinvert_ (Variables|Default|GetIsInvert?))
  (bind _ailerion_interior_rotation_max (Variables|MeshTransforms|GetAilerion%20Interior%20Rotation%20max))
  (bind _returnvalue_2 (Math|Float|SelectFloat -1.0 1.0 _isinvert_))
  (bind _returnvalue_3 (* AxisValue _returnvalue_2))
  ;[1 1 1] Look up input. Si no vuela haz la rotacion de la camara, si vuela rota el jet.
  (if (Variables|Default|GetIsFlying?)
    (bind _output_get (Variables|PlaneRotation|SetFlight%20Pitch (Math|Interpolation|FInterpTo (stale _output_get) _returnvalue_3 _returnvalue 0.0)))
    (Transformation|AddActorLocalRotation (Math|Rotator|MakeRotator 0.0 (* _output_get _returnvalue (Variables|PlaneRotation|GetFlight%20Turn%20Rate)) 0.0) false false)
    (Variables|MeshTransforms|SetAileron%20Interior%20Rotation (Math|Rotator|MakeRotator 0.0 (Math|Float|MapRangeClamped (Variables|PlaneRotation|GetFlight%20Pitch) -1.0 1.0 _ailerion_interior_rotation_max (* _ailerion_interior_rotation_max -1.0)) 0.0))
    (else
      (Pawn|Input|AddControllerPitchInput _returnvalue_3))))

(event Input|AxisEvents|InputAxisTurn
  (params (AxisValue :type Float%20%28single-precision%29))
  (bind _returnvalue (Utilities|Time|GetWorldDeltaSeconds))
  (bind _back_rudder_rotation_max (Variables|MeshTransforms|GetBack%20Rudder%20Rotation%20max))
  ;[1 1 1] Look up input. Si no vuela haz la rotacion de la camara, si vuela rota el jet.
  (if (Variables|Default|GetIsFlying?)
    (bind _output_get (Variables|PlaneRotation|SetFlight%20Turn (Math|Interpolation|FInterpTo (stale _output_get) AxisValue _returnvalue 0.0)))
    (Transformation|AddActorLocalRotation (Math|Rotator|MakeRotator 0.0 0.0 (* _output_get _returnvalue (Variables|PlaneRotation|GetFlight%20Turn%20Rate))) false false)
    (Variables|MeshTransforms|SetBack%20Rudder%20Rotation (Math|Rotator|MakeRotator 0.0 0.0 (Math|Float|MapRangeClamped (Variables|PlaneRotation|GetFlight%20Turn) -1.0 1.0 _back_rudder_rotation_max (* _back_rudder_rotation_max -1.0))))
    (else
      (Pawn|Input|AddControllerYawInput AxisValue))))

(event Input|AxisEvents|InputAxisMoveRight
  (params (AxisValue :type Float%20%28single-precision%29))
  (bind _ailerion_interior_rotation_max (Variables|MeshTransforms|GetAilerion%20Interior%20Rotation%20max))
  (bind _ailerion_interior_rotation_max_2 (Variables|MeshTransforms|GetAilerion%20Interior%20Rotation%20max))
  ;[1 1 1] Move Right input
  (if (Variables|Default|GetIsFlying?)
    (bind _output_get (Variables|PlaneRotation|SetFlight%20Roll (Math|Interpolation|FInterpTo (stale _output_get) AxisValue (Utilities|Time|GetWorldDeltaSeconds) 1e+01)))
    (Transformation|AddActorLocalRotation (Math|Rotator|MakeRotator (* _output_get (Utilities|Time|GetWorldDeltaSeconds) 9e+01) 0.0 0.0) false false)
    (Variables|MeshTransforms|SetAileron%20Flap%20Rotation%20Left (Math|Rotator|MakeRotator 0.0 (Math|Float|MapRangeClamped (Input|AxisValues|GetMoveRight) -1.0 1.0 _ailerion_interior_rotation_max_2 (* _ailerion_interior_rotation_max_2 -1.0)) 0.0))
    (Variables|MeshTransforms|SetAileron%20Flap%20Rotation%20Right (Math|Rotator|MakeRotator 0.0 (Math|Float|MapRangeClamped (Input|AxisValues|GetMoveRight) -1.0 1.0 (* _ailerion_interior_rotation_max -1.0) _ailerion_interior_rotation_max) 0.0))
    (else
      ;;[1 1 1] Que solo se pueda mover a izquierda o derecha mientras este en el suelo
      (if (> (Input|AxisValues|GetMoveForward) 0.0)
        (Class|Actor|AddActorWorldRotation (Math|Rotator|MakeRotator 0.0 0.0 (* AxisValue (Utilities|Time|GetWorldDeltaSeconds) 1e+01)))))))

(fn ConstructionScript)

(fn AddFlightMovement
  (bind _returnvalue (Utilities|Time|GetWorldDeltaSeconds))
  ;[1 1 1] Setado de la velocidad de vuelo
  (bind _output_get (Variables|Speed|SetCurrent%20thrust%20speed (Math|Interpolation|FInterpTo (stale _output_get) (Variables|Speed|GetTarget%20thrust%20speed) _returnvalue 8.0)))
  ;[1 1 1] Añadir moviemiento usando el forward
  (Transformation|AddActorWorldOffset (* (Math|Vector|GetForwardVector (Variables|Default|GetSK_West_Fighter_Typhoon)) (* _output_get _returnvalue)) true))

(fn LandingTrace
  (params (Debug :type EDrawDebugTrace%20Enum :default "None") (Spawned%20z%20offset :type Float%20%28double-precision%29))
  (bind _returnvalue (Transformation|GetActorLocation))
  (bind (_outhit _returnvalue_2) (Collision|LineTraceByChannel _returnvalue (- _returnvalue (Math|Vector|MakeVector 0.0 0.0 Spawned%20z%20offset)) "TraceTypeQuery1" false (Utilities|Array|MakeArray self) Debug))
  (if _returnvalue_2
    (if (< (Math|Float|MapRangeClamped (Variables|Speed|GetTarget%20thrust%20speed) (Variables|Speed|GetMinimum%20thrust%20speed) (Variables|Speed|GetMaximum%20thrust%20speed) 0.0 1.0) 0.5)
      (Variables|Default|SetIsFlying? false)
      (Transformation|SetActorRelativeTransform (Math|Transform|MakeTransform (Math|Interpolation|VInterpTo (Transformation|GetActorLocation) (+ (.TraceEnd (Collision|BreakHitResult _outhit)) (Math|Vector|MakeVector 0.0 0.0 Spawned%20z%20offset)) (Utilities|Time|GetWorldDeltaSeconds) 3.0) (Math|Rotator|MakeRotator 0.0 0.0 (.yaw (Transformation|GetActorRotation))) "1.000000,1.000000,1.000000") false false)
      (Variables|/Script/Engine.SpringArmComponent|SetbUsePawnControlRotation (Variables|Default|GetSpringArm) true)
      (Variables|Default|SetMove%20Forward%20Interp 1.0))))

(fn SetCameraLag
  (bind _springarm (Variables|Default|GetSpringArm))
  (bind _isflying_ (Variables|Default|GetIsFlying?))
  (bind _returnvalue (Math|Float|SelectFloat 1e+01 1e+03 _isflying_))
  ;[1 1 1] Si no estamos volando el lag deberia ser elevado
  (Variables|/Script/Engine.SpringArmComponent|SetCameraLagSpeed _springarm _returnvalue)
  (Variables|/Script/Engine.SpringArmComponent|SetCameraRotationLagSpeed _springarm _returnvalue))